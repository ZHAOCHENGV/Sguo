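; BP_Hero_Base is the base Blueprint for hero units, adding death handling for the hero's mount (坐骑) on top of its parent class.
; On death it runs the parent logic, then, if EnableRagdollOnDeath is set, switches the mount to physics-only ragdoll simulation.
; The same branch makes the mount, mesh and capsule ignore the Pawn channel.
; BeginPlay, Tick and construction only forward to the parent.
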(event EventBeginPlay
  (|CallParentFunction))

(event Collision|EventActorBeginOverlap
  (params (OtherActor :type Actor%20Object%20Reference))
  (|CallParentFunction OtherActor) ; 此节点被禁用，将不会被调用。\n从引脚连出引线来编译功能。
)

(event EventTick
  (params (DeltaSeconds :type Float%20%28single-precision%29))
  (|CallParentFunction DeltaSeconds))

(event EventOnDeath
  (bind _坐骑 (Variables|Default|Get坐骑))
  (|CallParentFunction)
  (if (Variables|Default|GetbEnableRagdollOnDeath)
    (Collision|SetCollisionProfileName _坐骑 "Ragdoll" true :!class /Script/Engine.PrimitiveComponent)
    (Collision|SetCollisionEnabled _坐骑 "PhysicsOnly")
    (Class|SkeletalMeshComponent|SetAllBodiesSimulatePhysics _坐骑 true)
    (Physics|SetSimulatePhysics _坐骑 true)
    (Collision|SetCollisionResponsetoChannel (Variables|Default|Get坐骑) "ECC_Pawn" "ECR_Ignore")))

(fn ConstructionScript
  (|CallParentFunction))