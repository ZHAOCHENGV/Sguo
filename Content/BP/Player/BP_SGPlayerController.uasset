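; Player controller that sets up the player's card deck and hand UI for the card system.
; On BeginPlay it waits briefly, initializes the CardDeckComponent and feeds it into the CardHandWidget, then binds the deck's selection and hand change events.
; Selection changes look up the card's detail info and print its name as debug text, while the hand change handler is still empty.
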(event Custom|OnSelectionChanged_事件
  (params (SelectedId :type Guid%20Structure%20%28by%20ref%29))
  (bind (_outdetailinfo _returnvalue) (Class|SGFunctionLibrary|GetCardDetailInfo (Variables|Default|GetCardDeckComponent) SelectedId))
  (if _returnvalue
    (Development|PrintString (Utilities|String|Append "当前选中的卡牌：" (Utilities|String|ToString(Text) (.CardName (Utilities|Struct|BreakSGCardDetailInfo _outdetailinfo)))) true true "(R=0.972904,G=1.000000,B=0.000000,A=1.000000)")))

(event Custom|OnHandChanged_事件
  (params (NewHand :type Array%20of%20SG%20Card%20Instance%20Structures)))

(event EventBeginPlay
  (bind _carddeckcomponent (Variables|Default|GetCardDeckComponent))
  (bind _carddeckcomponent_2 (Variables|Default|GetCardDeckComponent))
  (Utilities|FlowControl|Sequence
    (:then_0
      (Utilities|FlowControl|Delay 0.1)
      (Class|SGCardDeckComponent|InitializeDeck _carddeckcomponent_2)
      (Class|SGCardHandWidget|InitializeCardHand (Variables|Default|GetCardHandWidget) _carddeckcomponent_2))
    (:then_1
      (EventDispatchers|AssignOnSelectionChanged _carddeckcomponent (delegate Custom|OnSelectionChanged_事件))
      (EventDispatchers|AssignOnHandChanged _carddeckcomponent (delegate Custom|OnHandChanged_事件)))))

(event EventTick
  (params (DeltaSeconds :type Float%20%28single-precision%29)))

(fn ConstructionScript)