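; BP_TestGE is a test actor with a box volume that applies the GE_Test gameplay effect to overlapping BP_UnitBase actors.
; A short looping timer turns the box's collision off and straight back on, apparently to re-fire begin-overlap for units still inside.
; Each overlap builds the effect spec from the unit's own AbilitySystemComponent and applies it to itself, so the unit is both source and target.
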(event OnComponentBeginOverlap(Box)
  (params (OverlappedComponent :type Primitive%20Component%20Object%20Reference) (OtherActor :type Actor%20Object%20Reference) (OtherComp :type Primitive%20Component%20Object%20Reference) (OtherBodyIndex :type Integer) (bFromSweep :type Boolean) (SweepResult :type Hit%20Result%20Structure%20%28by%20ref%29))
  (bind _asbp_unit_base (Utilities|Casting|CastToBP_UnitBase OtherActor))
  (GameplayEffects|ApplyGameplayEffectSpecToTarget (Variables|/Script/Sguo.SG_UnitsBase|GetAbilitySystemComponent _asbp_unit_base) (GameplayEffects|MakeOutgoingSpec (Variables|/Script/Sguo.SG_UnitsBase|GetAbilitySystemComponent _asbp_unit_base) "/Game/BP/GAS/GE/GE_Test.GE_Test_C" 1.0 (GameplayEffects|MakeEffectContext (Variables|/Script/Sguo.SG_UnitsBase|GetAbilitySystemComponent _asbp_unit_base))) (Variables|/Script/Sguo.SG_UnitsBase|GetAbilitySystemComponent _asbp_unit_base)))

(event Custom|自定义事件
  (bind _box (Variables|Default|GetBox))
  (Collision|SetCollisionEnabled _box "NoCollision")
  (Collision|SetCollisionEnabled _box "QueryAndProbe"))

(event EventBeginPlay
  (Utilities|Time|SetTimerbyEvent (delegate Custom|自定义事件) 0.2 true))

(event Collision|EventActorBeginOverlap
  (params (OtherActor :type Actor%20Object%20Reference)))

(event EventTick
  (params (DeltaSeconds :type Float%20%28single-precision%29)))

(fn ConstructionScript)